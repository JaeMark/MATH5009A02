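; Game mode that tracks the player's score and runs the start and game-over flow.
; On BeginPlay it shows the score HUD and starts looping background music; UpdateScore adds a delta to Score and broadcasts it through the OnScoreUpdate dispatcher.
; HandlePlayerDeath pauses the game, swaps music for death sounds, and replaces the HUD with an end screen.
; The score is re-broadcast after each widget is created, supplying the current value.
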(event `self.ReceiveBeginPlay`
  (`|ExecutionSequence`
    (:`then_0`
      ;[1 1 1] Display score HUD
      (bind _returnvalue (`|CreateWidget` "/Game/MATH5009/Widgets/WBP_ScoreHUD.WBP_ScoreHUD_C"))
      (bind _output_get (set `self.ScoreHUD` _returnvalue))
      (`UserWidget.AddToViewport` _output_get 0))
    (:`then_1`
      (`self.OnScoreUpdate` (`self.Score`)))
    (:`then_2`
      (bind _returnvalue_2 (`GameplayStatics.SpawnSound2D` "/Game/MATH5009/Audio/War__Loop_.War__Loop_" 0.1 1.0 0.0 null))
      (set `self.BGMusic` _returnvalue_2))))

(event `/Game/MATH5009/Blueprints/BPI_ScoreHandler.UpdateScore`
  (params (DeltaScore :type "Float (double-precision)"))
  (bind _output_get (set `self.Score` (+ DeltaScore (`self.Score`))))
  (`self.OnScoreUpdate` _output_get))

(event `/Game/MATH5009/Blueprints/BPI_HandlePlayerDeath.HandlePlayerDeath`
  (`|ExecutionSequence`
    (:`then_0`
      (`GameplayStatics.SetGamePaused` true)
      (`AudioComponent.Stop` (`self.BGMusic`))
      (`GameplayStatics.PlaySound2D` "/Game/MATH5009/Audio/Church_Bell_2__loop_.Church_Bell_2__loop_" 0.2 1.0 0.0 null null)
      (`GameplayStatics.PlaySound2D` "/Game/MATH5009/Audio/Event12.Event12" 1.0 1.0 0.0 null null))
    (:`then_1`
      (`Widget.RemoveFromParent` (`self.ScoreHUD`)))
    (:`then_2`
      ;[1 1 1] Display end screen
      (bind _returnvalue (`|CreateWidget` "/Game/MATH5009/Widgets/WBP_EndScreen.WBP_EndScreen_C"))
      (`UserWidget.AddToViewport` _returnvalue 0)
      (`self.OnScoreUpdate` (`self.Score`)))))

(fn `UserConstructionScript`)