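; BP_HomingProjectile is a projectile that steers toward a Target and damages Enemy-tagged actors it overlaps, then destroys itself.
; After an initial delay, a looping timer snaps its yaw to face the target using atan2.
; Tick moves it along its forward vector in XY by Speed per frame, without delta-time scaling.
; An invalid target triggers a timer clear, but the misspelled "HomeToTarge" leaves the timer running.
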(event `self.ReceiveBeginPlay`
  (`KismetSystemLibrary.K2_SetTimer` null "HomeToTarget" 0.1 true (`self.DelayBeforeHomng`)))

(event `HomeToTarget`
  (bind (_returnvalue_x _returnvalue_y) (`KismetMathLibrary.BreakVector` (- (`self.K2_GetActorLocation` (`self.Target`)) (`self.K2_GetActorLocation`))))
  (`/Engine/EditorBlueprintResources/StandardMacros.IsValid` (`self.Target`)
    (:`Is Valid`
      (`self.K2_SetActorRotation` (`KismetMathLibrary.MakeRotator` 0.0 0.0 (`KismetMathLibrary.DegAtan2` _returnvalue_y _returnvalue_x))))
    (:`Is Not Valid`
      (`KismetSystemLibrary.K2_ClearTimer` null "HomeToTarge"))))

(event `self.ReceiveTick`
  (params (DeltaSeconds :type "Float (single-precision)"))
  (bind (_returnvalue_x _returnvalue_y) (`KismetMathLibrary.BreakVector` (* (`self.GetActorForwardVector`) (`self.Speed`))))
  (`self.K2_AddActorWorldOffset` (`KismetMathLibrary.MakeVector` _returnvalue_x _returnvalue_y)))

(event `self.SphereCollider.OnComponentBeginOverlap`
  (params (OverlappedComponent :type "PrimitiveComponent Object Reference") (OtherActor :type "Actor Object Reference") (OtherComp :type "PrimitiveComponent Object Reference") (OtherBodyIndex :type Integer) (bFromSweep :type Boolean) (SweepResult :type "HitResult Structure (by ref)"))
  (if (`self.ActorHasTag` OtherActor "Enemy")
    (`GameplayStatics.ApplyDamage` OtherActor (`self.Damage`) null self)
    (`self.K2_DestroyActor`)))

(fn `UserConstructionScript`)