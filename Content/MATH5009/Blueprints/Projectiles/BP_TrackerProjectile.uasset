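; BP_TrackerProjectile is a colored projectile that damages actors tagged "Enemy"; despite its name, it contains no homing logic.
; Tick offsets it along its forward vector in X and Y only, scaled by Speed without delta time.
; An enemy overlap applies damage and destroys it with a hit effect, as does a Lifetime timer without the damage.
; The construction script and hit effects share one Color variable for particle tinting.
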(event `self.ReceiveBeginPlay`
  (`KismetSystemLibrary.K2_SetTimer` null "DestroyProjectile" (`self.Lifetime`)))

(event `DestroyProjectile`
  (bind (_returnvalue_location _returnvalue_rotation _returnvalue_scale) (`KismetMathLibrary.BreakTransform` (`SceneComponent.K2_GetComponentToWorld` (`self.Projectile`))))
  (bind _returnvalue (`GameplayStatics.SpawnEmitterAtLocation` "/Game/MagicProjectilesVol2/Particles/Hits/P_Hit_Orb01_Purple.P_Hit_Orb01_Purple" _returnvalue_location _returnvalue_rotation _returnvalue_scale))
  (`FXSystemComponent.SetColorParameter` _returnvalue "Color" (`self.Color`))
  (`self.K2_DestroyActor`))

(event `self.SphereCollider.OnComponentBeginOverlap`
  (params (OverlappedComponent :type "PrimitiveComponent Object Reference") (OtherActor :type "Actor Object Reference") (OtherComp :type "PrimitiveComponent Object Reference") (OtherBodyIndex :type Integer) (bFromSweep :type Boolean) (SweepResult :type "HitResult Structure (by ref)"))
  (bind (_returnvalue_location _returnvalue_rotation _returnvalue_scale) (`KismetMathLibrary.BreakTransform` (`SceneComponent.K2_GetComponentToWorld` (`self.Projectile`))))
  (if (`self.ActorHasTag` OtherActor "Enemy")
    (`GameplayStatics.ApplyDamage` OtherActor (`self.Damage`) (`Pawn.GetController` (`self.GetInstigator`)) self)
    (bind _returnvalue (`GameplayStatics.SpawnEmitterAtLocation` "/Game/MagicProjectilesVol2/Particles/Hits/P_Hit_Orb01_Purple.P_Hit_Orb01_Purple" (`self.K2_GetActorLocation` OtherActor) _returnvalue_rotation _returnvalue_scale))
    (`FXSystemComponent.SetColorParameter` _returnvalue "Color" (`self.Color`))
    (`self.K2_DestroyActor`)))

(event `self.ReceiveTick`
  (params (DeltaSeconds :type "Float (single-precision)"))
  (bind (_returnvalue_x _returnvalue_y) (`KismetMathLibrary.BreakVector` (* (`self.GetActorForwardVector`) (`self.Speed`))))
  (`self.K2_AddActorWorldOffset` (`KismetMathLibrary.MakeVector` _returnvalue_x _returnvalue_y)))

(fn `UserConstructionScript`
  (bind _color (`self.Color`))
  (`FXSystemComponent.SetColorParameter` (`self.Projectile`) "Color" _color)
  (`FXSystemComponent.SetColorParameter` (`self.Muzzle`) "Color" _color))