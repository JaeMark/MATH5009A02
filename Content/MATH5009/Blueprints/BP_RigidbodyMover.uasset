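; BP_RigidbodyMover is a helper that moves its owning actor by an offset only when the path is clear.
; InitializeCollider stores the collider radius, blocking object types and ignored actors.
; AddWorldOffset calls CheckIfBlocked, which sphere-traces from the owner's location along the offset with one-frame debug drawing.
; If nothing is hit, it applies the offset without sweep and returns true; otherwise it returns false.
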(fn `AddWorldOffset`
  (params (LocationOffset :type "Vector Structure"))
  (returns (bIsBlocked :type Boolean))
  (bind _bisblocked (`self.CheckIfBlocked` LocationOffset))
  (if (not _bisblocked)
    (`Actor.K2_AddActorWorldOffset` (`self.GetOwner`) LocationOffset false false)
    (return true)
    (else
      (return false))))

(fn `CheckIfBlocked`
  (params (Offset :type "Vector Structure"))
  (returns (bIsBlocked :type Boolean))
  (bind _returnvalue (`Actor.K2_GetActorLocation` (`self.GetOwner`)))
  (bind (_outhits _returnvalue_2) (`KismetSystemLibrary.SphereTraceMultiForObjects` _returnvalue (+ _returnvalue (`local.Offset`)) (`self.ColliderRadius`) (`self.BlockedObjectType`) false (`self.ActorsToIgnore`) "ForOneFrame"))
  (return _returnvalue_2))

(fn `InitializeCollider`
  (params (ColliderRadius :type "Float (double-precision)") (BlockedObjectType :type "Array of EObjectTypeQuery Enum") (ActorsToIgnore :type "Array of Actor Object Reference"))
  (set `self.ColliderRadius` ColliderRadius)
  (set `self.BlockedObjectType` BlockedObjectType)
  (set `self.ActorsToIgnore` ActorsToIgnore))