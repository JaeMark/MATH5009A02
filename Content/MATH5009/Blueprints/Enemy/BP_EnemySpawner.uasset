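; Enemy spawner actor that periodically creates BP_Enemy instances inside a box volume.
; On BeginPlay a looping timer calls SpawnEnemy at the spawn interval.
; Each call counts all BP_Enemy actors in the world and, while below the maximum, spawns one at a random XY point within SpawnCollider.
; Spawn Z is set to the enemy collider half height rather than taken from the box.
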(event `self.ReceiveBeginPlay`
  (`KismetSystemLibrary.K2_SetTimer` null "SpawnEnemy" (`self.SpawnInterval`) true))

(event `SpawnEnemy`
  (bind (_returnvalue_x _returnvalue_y) (`KismetMathLibrary.BreakVector` (`KismetMathLibrary.RandomPointInBoundingBox` (`SceneComponent.K2_GetComponentLocation` (`self.SpawnCollider`)) (`BoxComponent.GetScaledBoxExtent` (`self.SpawnCollider`)))))
  (bind _outactors (`GameplayStatics.GetAllActorsOfClass` "/Game/MATH5009/Blueprints/Enemy/BP_Enemy.BP_Enemy_C"))
  (if (< (`KismetArrayLibrary.Array_Length` _outactors) (`self.MaxEnemies`))
    (`|SpawnActorFromClass` "/Game/MATH5009/Blueprints/Enemy/BP_Enemy.BP_Enemy_C" (`KismetMathLibrary.MakeTransform` (`KismetMathLibrary.MakeVector` _returnvalue_x _returnvalue_y (`self.EnemyColliderHalfHeight`))) "Undefined" "MultiplyWithRoot" null null)))

(fn `UserConstructionScript`)