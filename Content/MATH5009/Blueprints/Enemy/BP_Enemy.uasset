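; Enemy actor that pursues the player, spits projectiles at attackable targets ahead and deals contact damage.
; A looping timeline eases its yaw toward the player while Tick moves it forward through BPRigidbodyMover.
; A forward sphere trace pauses movement for a spit montage, whose notify spawns the projectile.
; Damage from tracker projectiles reports it to the shooter as a track target, and death updates the GameMode score before delayed destruction.
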(event `self.ReceiveBeginPlay`
  (set `self.Health` (`self.MaxHealth`))
  (`/Game/MATH5009/Blueprints/BPC_RigidbodyMover.InitializeCollider` (`self.BP_RigidbodyMover`) (`CapsuleComponent.GetScaledCapsuleRadius` (`self.Collider`)) (`self.Blocked Object Type`) (`|MakeArray` self :!type "Actor Object Reference"))
  (`self.FaceTarget`))

(event `self.ReceiveTick`
  (params (DeltaSeconds :type "Float (single-precision)"))
  (bind _returnvalue (`self.K2_GetActorLocation`))
  (bind (_returnvalue_location _returnvalue_rotation) (`KismetMathLibrary.BreakTransform` (`SceneComponent.K2_GetComponentToWorld` (`self.MouthProjectileArrow`))))
  (bind (_returnvalue_x _returnvalue_y) (`KismetMathLibrary.BreakVector` (* (`KismetMathLibrary.Conv_RotatorToVector` (`self.K2_GetActorRotation`)) (`self.MovementSpeed`))))
  (if (not (`self.bIsDead`))
    (`|ExecutionSequence`
      (:`then_0`
        (if (not (`self.bIsAttacking`))
          ;[1 1 1] Check if attackable actor is within range
          (bind (_outhit _returnvalue_2) (`KismetSystemLibrary.SphereTraceSingleForObjects` :`Start` _returnvalue :`End` (+ _returnvalue (* (`KismetMathLibrary.Conv_RotatorToVector` (`self.K2_GetActorRotation`)) (`self.AttackRange`))) :`Radius` (`self.AttackRadius`) :`ObjectTypes` (`self.AttackableObjectType`) :`TraceColor` (struct :`G` 0.063052 :`B` 1.0 :`A` 1.0) :`TraceHitColor` (struct :`R` 1.0 :`G` 0.948144 :`A` 1.0)))
          (if _returnvalue_2
            (set `self.bIsAttacking` true)
            ;[1 1 1] Play attack animation and spawn attack projectile
            (`|PlayMontage` (`self.SkeletalMesh`) "/Game/MATH5009/Animation/Enemy/AM_Spit.AM_Spit" 2.0
              (:`OnCompleted`
                (set `self.bIsAttacking` false))
              (:`OnNotifyBegin`
                (`|SpawnActorFromClass` "/Game/MATH5009/Blueprints/Projectiles/BP_EnemyProjectile.BP_EnemyProjectile_C" (`KismetMathLibrary.MakeTransform` _returnvalue_location _returnvalue_rotation) "Undefined" "MultiplyWithRoot" null (`self.ProjectileLifetime`) null))))))
      (:`then_1`
        ;[1 1 1] Move actor forward
        (if (not (`self.bIsAttacking`))
          (bind _bisblocked (`/Game/MATH5009/Blueprints/BPC_RigidbodyMover.AddWorldOffset` (`self.BP_RigidbodyMover`) (`KismetMathLibrary.MakeVector` _returnvalue_x _returnvalue_y)))
          (set `self.bIsMoving` (not _bisblocked)))))))

(event `FaceTarget`
  (bind (_returnvalue_x _returnvalue_y) (`KismetMathLibrary.BreakVector` (- (`self.K2_GetActorLocation`) (`self.K2_GetActorLocation` (`GameplayStatics.GetPlayerPawn` 0)))))
  (if (not (`self.bIsDead`))
    (set `self.InitialPlayerRotation` (`self.K2_GetActorRotation`))
    (bind (_direction _newtrack_0) (`Timeline|RotationalEasingTimeline` :!via `PlayFromStart`)
      (:`Update`
        (`self.K2_SetActorRotation` (`KismetMathLibrary.RLerp` (`self.InitialPlayerRotation`) (`KismetMathLibrary.RotatorFromAxisAndAngle` (0.0 0.0 1.0) (+ (`KismetMathLibrary.DegAtan2` _returnvalue_y _returnvalue_x) 180.0)) _newtrack_0 true)))
      (:`Finished`
        (`KismetSystemLibrary.Delay` 0.2)
        (`self.FaceTarget`)))))

(event `self.ReceiveAnyDamage`
  (params (Damage :type "Float (single-precision)") (DamageType :type "DamageType Object Reference") (InstigatedBy :type "Controller Object Reference") (DamageCauser :type "Actor Object Reference"))
  (bind _output_get (set `self.Health` (`KismetMathLibrary.FClamp` (- (`self.Health`) Damage) 0.0 (`self.MaxHealth`))))
  (if (<= _output_get 0.0)
    ;[1 1 1] Handle actor death
    (`/Engine/EditorBlueprintResources/StandardMacros.DoOnce` false
      (:`Completed`
        (set `self.bIsDead` true)
        (message `/Game/MATH5009/Blueprints/BPI_ScoreHandler.UpdateScore` (`GameplayStatics.GetGameMode`) (`self.Score`))
        (`KismetSystemLibrary.Delay` 2.0)
        (`self.K2_DestroyActor`)))
    (else
      ;[1 1 1] Apply tracker on this actor if hit by tracker projectile
      (if (`self.ActorHasTag` DamageCauser "TrackerProjectile")
        (message `/Game/MATH5009/Blueprints/BPI_Tracker.OnTrackTargetSet` (`Controller.K2_GetPawn` InstigatedBy) self)))))

(event `self.Collider.OnComponentBeginOverlap`
  (params (OverlappedComponent :type "PrimitiveComponent Object Reference") (OtherActor :type "Actor Object Reference") (OtherComp :type "PrimitiveComponent Object Reference") (OtherBodyIndex :type Integer) (bFromSweep :type Boolean) (SweepResult :type "HitResult Structure (by ref)"))
  ;[1 1 1] Apply damage to the player on close contact
  (`/Engine/EditorBlueprintResources/StandardMacros.IsValid` OtherActor
    (:`Is Valid`
      (if (`self.ActorHasTag` OtherActor "Player")
        (`GameplayStatics.ApplyDamage` OtherActor (`self.ContactDamage`))))))

(event `/Game/MATH5009/Blueprints/BPI_Trackable.RemoveTracker`
  (`ActorComponent.K2_DestroyComponent` (`self.TrackerIndicator`)))

(event `/Game/MATH5009/Blueprints/BPI_Trackable.SetTracker`
  (params (Tracker :type "ActorComponent Object Reference"))
  (set `self.TrackerIndicator` Tracker))

(fn `UserConstructionScript`)