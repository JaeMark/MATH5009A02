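; BP_Enemy is an enemy actor that chases the player and can take damage.
; Each tick it yaws toward the player pawn and feeds a horizontal forward offset, not scaled by delta time, to BPRigidbodyMover, initialized with its capsule radius.
; AnyDamage lowers clamped health and destroys the actor one second after it reaches zero.
; Surviving hits from TrackerProjectile-tagged causers message the instigator's pawn to set this enemy as track target.
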(event `self.ReceiveTick`
  (params (DeltaSeconds :type "Float (single-precision)"))
  (bind (_returnvalue_x _returnvalue_y) (`KismetMathLibrary.BreakVector` (- (`self.K2_GetActorLocation`) (`self.K2_GetActorLocation` (`GameplayStatics.GetPlayerPawn` 0)))))
  (bind (_returnvalue_x_2 _returnvalue_y_2) (`KismetMathLibrary.BreakVector` (* (`KismetMathLibrary.Conv_RotatorToVector` (`self.K2_GetActorRotation`)) (`self.MovementSpeed`))))
  (`|ExecutionSequence`
    (:`then_0`
      (`self.K2_SetActorRotation` (`KismetMathLibrary.MakeRotator` 0.0 0.0 (+ (`KismetMathLibrary.DegAtan2` _returnvalue_y _returnvalue_x) 180.0))))
    (:`then_1`
      (`/Game/MATH5009/Blueprints/BP_RigidbodyMover.AddWorldOffset` (`self.BP_RigidbodyMover`) (`KismetMathLibrary.MakeVector` _returnvalue_x_2 _returnvalue_y_2)))))

(event `self.ReceiveBeginPlay`
  (set `self.Health` (`self.MaxHealth`))
  (`/Game/MATH5009/Blueprints/BP_RigidbodyMover.InitializeCollider` (`self.BP_RigidbodyMover`) (`CapsuleComponent.GetScaledCapsuleRadius` (`self.Collider`)) (`self.Blocked Object Type`) (`|MakeArray` self)))

(event `self.ReceiveAnyDamage`
  (params (Damage :type "Float (single-precision)") (DamageType :type "DamageType Object Reference") (InstigatedBy :type "Controller Object Reference") (DamageCauser :type "Actor Object Reference"))
  (bind _output_get (set `self.Health` (`KismetMathLibrary.FClamp` (- (`self.Health`) Damage) 0.0 (`self.MaxHealth`))))
  (if (<= _output_get 0.0)
    (`KismetSystemLibrary.Delay` 1.0)
    (`self.K2_DestroyActor`)
    (elif (`self.ActorHasTag` DamageCauser "TrackerProjectile")
      (message `/Game/MATH5009/Blueprints/BPI_OnTrackStatusSet.OnTrackTargetSet` (`Controller.K2_GetPawn` InstigatedBy) self))))

(fn `UserConstructionScript`)